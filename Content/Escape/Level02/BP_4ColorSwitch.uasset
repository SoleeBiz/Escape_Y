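; BP_4ColorSwitch is an interactable four-color switch puzzle for Level02 of the Escape game.
; Overlapping its box shows a text prompt and enables input, letting F open the BP_SwitchUI widget in UI-only mode.
; The widget's submitted answer is compared with CorrectAnswer, firing right or wrong dispatchers, the former intended for Level Blueprint binding.
; Only a wrong answer clears the UI-shown flag, allowing a retry.
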(event OnComponentBeginOverlap(Box)
  (params (OverlappedComponent :type Primitive%20Component%20Object%20Reference) (OtherActor :type Actor%20Object%20Reference) (OtherComp :type Primitive%20Component%20Object%20Reference) (OtherBodyIndex :type Integer) (bFromSweep :type Boolean) (SweepResult :type Hit%20Result%20Structure%20%28by%20ref%29))
  ;[1 1 1] Press F Key txt
  (Rendering|SetVisibility (Variables|Default|GetTextRender) true false)
  (Input|EnableInput (Game|GetPlayerController 0)))

(event OnComponentEndOverlap(Box)
  (params (OverlappedComponent :type Primitive%20Component%20Object%20Reference) (OtherActor :type Actor%20Object%20Reference) (OtherComp :type Primitive%20Component%20Object%20Reference) (OtherBodyIndex :type Integer))
  ;[1 1 1] Press F Key txt
  (Rendering|SetVisibility (Variables|Default|GetTextRender) false false)
  (Input|DisableInput (Game|GetPlayerController 0)))

(event Custom|OnUserAnswer
  (params (UserInput :type Integer))
  (if (== UserInput (Variables|Default|GetCorrectAnswer))
    (Default|CallOnAnswerIsRight UserInput) ; 레벨 블루프린트에서 바인딩
    (else
      (Default|CallOnAnswerIsWrong UserInput)
      (Variables|Default|SetIsShowUI false))))

(event EventBeginPlay
  (Utilities|FlowControl|Sequence
    (:then_0
      (bind _returnvalue (UserInterface|CreateWidget "/Game/Escape/Level02/BP_SwitchUI.BP_SwitchUI_C"))
      (Variables|Default|SetSwitchUI _returnvalue))
    (:then_1
      (EventDispatchers|BindEventtoOnUserAnswer (Variables|Default|GetSwitchUI) (delegate Custom|OnUserAnswer)) ; WIDGET 생성한 곳에서 바인딩 해줘야 함
    )))

(event Input|KeyboardEvents|F
  (params (Key :type Key%20Structure :default "None"))
  (bind _returnvalue (Game|GetPlayerController 0))
  ;[1 1 1] Show UI
  (:Released
    (if (not (Variables|Default|GetIsShowUI))
      (UserInterface|Viewport|AddtoViewport (Variables|Default|GetSwitchUI) 0)
      (Variables|Default|SetIsShowUI true)
      (Variables|/Script/Engine.PlayerController|SetbShowMouseCursor _returnvalue true)
      (Input|SetInputModeUIOnly _returnvalue 0 "DoNotLock"))))

(fn ConstructionScript)